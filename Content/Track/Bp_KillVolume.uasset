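; Kill volume for the track that triggers the player's death when their pawn overlaps it.
; It caches the first SportsCar_Pawn found at BeginPlay and checks overlaps against player 0's pawn.
; On a match, it applies DAMAGE to the cached car, not the overlapping actor, then calls HandlePlayerDeath on it regardless of the damage result.
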(event `self.ReceiveBeginPlay`
  (bind _returnvalue (`GameplayStatics.GetActorOfClass` "/Game/VehicleTemplate/Blueprints/SportsCar/SportsCar_Pawn.SportsCar_Pawn_C"))
  (set `self.Playerref` _returnvalue))

(event `self.ReceiveActorBeginOverlap`
  (params (OtherActor :type "Actor Object Reference"))
  (if (== OtherActor (`GameplayStatics.GetPlayerPawn` 0))
    (`GameplayStatics.ApplyDamage` (`self.Playerref`) (`self.DAMAGE `))
    (`/Game/VehicleTemplate/Blueprints/SportsCar/SportsCar_Pawn.Handle player Death` (`self.Playerref`))))

(fn `UserConstructionScript`)