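; Trigger actor on the track that swaps the player's car model, likely as part of a world change.
; On BeginPlay it caches the level's SportsCar_Pawn as the player reference.
; When the player pawn stops overlapping it, it replaces that car's skeletal mesh and anim class with the configured NewMesh and NewAnimation.
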(event `self.ReceiveBeginPlay`
  (bind _returnvalue (`GameplayStatics.GetActorOfClass` "/Game/VehicleTemplate/Blueprints/SportsCar/SportsCar_Pawn.SportsCar_Pawn_C"))
  (set `self.PLayerref` _returnvalue))

(event `self.ReceiveActorEndOverlap`
  (params (OtherActor :type "Actor Object Reference"))
  (bind _mesh (`WheeledVehiclePawn.Mesh` (`self.PLayerref`)))
  (if (== OtherActor (`GameplayStatics.GetPlayerPawn` 0))
    (`SkeletalMeshComponent.SetSkeletalMeshAsset` _mesh (`self.New Mesh`))
    (`SkeletalMeshComponent.SetAnimInstanceClass` _mesh (`self.New animation`))))

(fn `UserConstructionScript`)